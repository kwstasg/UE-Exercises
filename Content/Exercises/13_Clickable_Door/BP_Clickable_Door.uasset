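; BP_Clickable_Door is a door that opens once it has been clicked and an actor is in its trigger Box.
; Hovering the Cube switches the mouse cursor to a hand.
; A click opens it at once if Exercise_13_Character overlaps the Box, otherwise the stored Clicked flag opens it on the next overlap.
; A Timeline slides the Cube along relative Z and reverses when an overlap ends.
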(event OnBeginCursorOver(Cube)
  (params (TouchedComponent :type Primitive%20Component%20Object%20Reference))
  (Variables|/Script/Engine.PlayerController|SetCurrentMouseCursor (Game|GetPlayerController 0) "Hand"))

(event OnEndCursorOver(Cube)
  (params (TouchedComponent :type Primitive%20Component%20Object%20Reference))
  (Variables|/Script/Engine.PlayerController|SetCurrentMouseCursor (Game|GetPlayerController 0) "Default"))

(event OnClicked(Cube)
  (params (TouchedComponent :type Primitive%20Component%20Object%20Reference) (ButtonPressed :type Key%20Structure :default "None"))
  (Variables|Default|SetClicked true)
  (bind _returnvalue (Actor|GetActorOfClass "/Game/Exercises/13_Clickable_Door/Exercise_13_Character.Exercise_13_Character_C"))
  (if (Collision|IsOverlappingActor (Variables|Default|GetBox) _returnvalue :!class /Script/Engine.PrimitiveComponent)
    (Variables|Default|SetClicked false)
    (bind _door_z (Timeline|Timeline Play)
      (:Update
        (Transformation|SetRelativeLocation (Variables|Default|GetCube) (Math|Vector|MakeVector 5e+01 2e+02 _door_z) false false)))))

(event Collision|EventActorBeginOverlap
  (params (OtherActor :type Actor%20Object%20Reference))
  (if (Variables|Default|GetClicked)
    (Variables|Default|SetClicked false)
    (bind _door_z (Timeline|Timeline Play)
      (:Update
        (Transformation|SetRelativeLocation (Variables|Default|GetCube) (Math|Vector|MakeVector 5e+01 2e+02 _door_z) false false)))))

(event Collision|EventActorEndOverlap
  (params (OtherActor :type Actor%20Object%20Reference))
  (bind _door_z (Timeline|Timeline Reverse)
    (:Update
      (Transformation|SetRelativeLocation (Variables|Default|GetCube) (Math|Vector|MakeVector 5e+01 2e+02 _door_z) false false))))

(fn ConstructionScript)