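; BP_Events_Order is an exercise Blueprint that prints on-screen messages to show when common events fire.
; It logs the Construction Script, BeginPlay, begin and end overlaps, and Tick, with Tick output gated by the TickDebug flag.
; Hardcoded key, mouse button, wheel and mouse XY events also print, relying on Auto Receive Input set to Player 0, with XY output gated by MouseDebug.
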(event EventBeginPlay
  ;[0 0.15 0.03663 0.5] On Game/Level Start
  (Development|PrintString "Event BeginPlay Fired" true true "(R=0.000000,G=0.660000,B=1.000000,A=1.000000)" 5.0))

(event Collision|EventActorBeginOverlap
  (params (OtherActor :type Actor%20Object%20Reference))
  ;[0.15 0.03509 0.07796 0.5] On Collision
  (Development|PrintText (Utilities|Text|FormatText "Event Begin Overlap Fired Other Actor: {0}" OtherActor)))

(event EventTick
  (params (DeltaSeconds :type Float%20%28single-precision%29))
  ;[0 0.04238 0.15 0.5] On Every Frame
  (if (Variables|Default|GetTick%20Debug)
    (Development|PrintText (Utilities|Text|FormatText "Event Tick Fired Delta Seconds: {0}" DeltaSeconds))))

(event Collision|EventActorEndOverlap
  (params (OtherActor :type Actor%20Object%20Reference))
  ;[0.15 0.03509 0.07796 0.5] On Collision
  (Development|PrintText (Utilities|Text|FormatText "Event End Overlap Fired Other Actor: {0}" OtherActor)))

(event Input|MouseEvents|MouseWheelAxis
  (params (AxisValue :type Float%20%28single-precision%29))
  ;[0.15 0.1382 0.05187 0.5] Hardcoded Input (Auto Receive input must be set to Player 0 in Class Defaults)
  (if (!= AxisValue 0.0)
    (Development|PrintText (Utilities|Text|FormatText "Mouse Wheel Axis Value: {0}" AxisValue))))

(event Input|KeyboardEvents|1
  (params (Key :type Key%20Structure :default "None"))
  ;[0.15 0.1382 0.05187 0.5] Hardcoded Input (Auto Receive input must be set to Player 0 in Class Defaults)
  (:Pressed
    (Development|PrintText (Utilities|Text|FormatText "Key 1 Pressed")))
  (:Released
    (Development|PrintText (Utilities|Text|FormatText "Key 1 Relesed"))))

(event Input|MouseEvents|LeftMouseButton
  (params (Key :type Key%20Structure :default "None"))
  ;[0.15 0.1382 0.05187 0.5] Hardcoded Input (Auto Receive input must be set to Player 0 in Class Defaults)
  (:Pressed
    (Development|PrintText (Utilities|Text|FormatText "Left Click Pressed")))
  (:Released
    (Development|PrintText (Utilities|Text|FormatText "Left Click Relesed"))))

(event Input|MouseEvents|Mouse2D
  (params (AxisValue :type Vector :default "0, 0, 0"))
  ;[0.15 0.1382 0.05187 0.5] Hardcoded Input (Auto Receive input must be set to Player 0 in Class Defaults)
  (if (Variables|Default|GetMouse%20Debug)
    (Development|PrintText (Utilities|Text|FormatText "Mouse XY Axis Value: {0} {1}" (.x AxisValue) (.y AxisValue)))))

(fn ConstructionScript
  (Development|PrintString "Construction Script Fired" true true "(R=0.000000,G=0.660000,B=1.000000,A=1.000000)" 5.0))